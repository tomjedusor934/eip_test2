(event Input|EnhancedActionEvents|EnhancedInputActionIA_Confirm
  (params (ActionValue :type Boolean) (ElapsedSeconds :type Float%20%28double-precision%29) (TriggeredSeconds :type Float%20%28double-precision%29) (InputAction :type Input%20Action%20Object%20Reference :default "/Game/Game/Blueprint/Inputs/IA_Confirm.IA_Confirm"))
  (:Started
    (Variables|Default|GetItemToBuild
      (:then
        (CallFunction|PlaceBuild))
      (:else
        (bind _itemtodelete (Variables|Default|GetItemToDelete)
          (:then
            (Default|DestroyBuild _itemtodelete))
          (:else))))))

(event Input|EnhancedActionEvents|EnhancedInputActionIA_Deconstruct
  (params (ActionValue :type Boolean) (ElapsedSeconds :type Float%20%28double-precision%29) (TriggeredSeconds :type Float%20%28double-precision%29) (InputAction :type Input%20Action%20Object%20Reference :default "/Game/Game/Blueprint/Inputs/IA_Deconstruct.IA_Deconstruct"))
  (:Started
    (if (Utilities|Time|IsValidTimerHandle (Variables|Default|GetDeleteBuild))
      (bind _itemtodelete (Variables|Default|GetItemToDelete)
        (:then
          (Default|SetAllMaterials _itemtodelete 0 true)
          (Variables|Default|SetItemToDelete 0))
        (:else
          _))
      (Utilities|Time|ClearandInvalidateTimerbyHandle (Variables|Default|GetDeleteBuild))
      (else
        (Variables|Default|GetItemToBuild
          (:then
            (CallFunction|CancelBuild))
          (:else
            _))
        (bind _returnvalue (Utilities|Time|SetTimerbyFunctionName 0 "DetermineDelete" 0.05 true))
        (Variables|Default|SetDeleteBuild _returnvalue)))))

(event Input|EnhancedActionEvents|EnhancedInputActionIA_Scroll
  (params (ActionValue :type Float%20%28double-precision%29) (ElapsedSeconds :type Float%20%28double-precision%29) (TriggeredSeconds :type Float%20%28double-precision%29) (InputAction :type Input%20Action%20Object%20Reference :default "/Game/Game/Blueprint/Inputs/IA_Scroll.IA_Scroll"))
  (bind _itemtobuild (Variables|Default|GetItemToBuild)
    (:then
      (if (Variables|Default|GetIsCtrlDown)
        (Default|ScrollBuildCustom _itemtobuild ActionValue)
        (else
          (Default|ScrollBuild _itemtobuild ActionValue))))
    (:else)))

(event Input|EnhancedActionEvents|EnhancedInputActionIA_Object1
  (params (ActionValue :type Boolean) (ElapsedSeconds :type Float%20%28double-precision%29) (TriggeredSeconds :type Float%20%28double-precision%29) (InputAction :type Input%20Action%20Object%20Reference :default "/Game/Game/Blueprint/Inputs/IA_Object1.IA_Object1"))
  (:Started
    (CallFunction|SpawnBuild "/Game/Game/Blueprint/A_Builds_Support.A_Builds_Support_C")))

(event Input|EnhancedActionEvents|EnhancedInputActionIA_Interact
  (params (ActionValue :type Boolean) (ElapsedSeconds :type Float%20%28double-precision%29) (TriggeredSeconds :type Float%20%28double-precision%29) (InputAction :type Input%20Action%20Object%20Reference :default "/Game/Game/Blueprint/Inputs/IA_Interact.IA_Interact"))
  (:Started
    (bind (_outhit _returnvalue) (CallFunction|LineTracefromCamera "TraceTypeQuery1"))
    (if _returnvalue
      (if (Utilities|DoesObjectImplementInterface (.HitActor (Collision|BreakHitResult _outhit)) "/Game/Game/Blueprint/BPI_interaction.BPI_interaction_C")
        (Class|BPIInteraction|InteractWitchActor(Message) (.HitActor (Collision|BreakHitResult _outhit)))))))

(event Input|EnhancedActionEvents|EnhancedInputActionIA_Object2
  (params (ActionValue :type Boolean) (ElapsedSeconds :type Float%20%28double-precision%29) (TriggeredSeconds :type Float%20%28double-precision%29) (InputAction :type Input%20Action%20Object%20Reference :default "/Game/Game/Blueprint/Inputs/IA_Object2.IA_Object2"))
  (:Started
    (CallFunction|SpawnBuild "/Game/Game/Blueprint/A_Builds_Conveyer.A_Builds_Conveyer_C")))

(event EventBeginPlay
  (Input|AddMappingContext (PlayerController|LocalPlayerSubsystems|GetEnhancedInputLocalPlayerSubsystem (Game|GetPlayerController 0)) "/Game/Game/Blueprint/Inputs/IMC_satisfactory.IMC_satisfactory" 0 "(bIgnoreAllPressedKeysUntilRelease=True,bForceImmediately=False,bNotifyUserSettings=False)")
  (bind _returnvalue (UserInterface|CreateWidget "/Game/Game/Widgets/NewWidgetBlueprint.NewWidgetBlueprint_C"))
  (UserInterface|Viewport|AddtoViewport _returnvalue 0)
  (bind _returnvalue_2 (UserInterface|CreateWidget "/Game/Game/Widgets/inventory/WB_Interact.WB_Interact_C"))
  (bind _output_get (Variables|Default|SetInteractWidget _returnvalue_2))
  (UserInterface|Viewport|AddtoViewport _output_get 0)
  (Widget|SetVisibility _output_get "Collapsed"))

(event EventTick
  (params (DeltaSeconds :type Float%20%28single-precision%29))
  (bind _interactwidget (Variables|Default|GetInteractWidget))
  (bind (_outhit _returnvalue) (CallFunction|LineTracefromCamera "TraceTypeQuery1"))
  (if _returnvalue
    (if (Utilities|DoesObjectImplementInterface (.HitActor (Collision|BreakHitResult _outhit)) "/Game/Game/Blueprint/BPI_interaction.BPI_interaction_C")
      (if (!= (Variables|Default|GetPreviouslyOverlapActor) (.HitActor (Collision|BreakHitResult _outhit)))
        (Class|BPIInteraction|OverlapInteraction(Message) (.HitActor (Collision|BreakHitResult _outhit)) _interactwidget)
        (Variables|Default|SetPreviouslyOverlapActor (.HitActor (Collision|BreakHitResult _outhit)))
        (Widget|SetVisibility _interactwidget "Visible"))
      (else
        (Widget|SetVisibility (Variables|Default|GetInteractWidget) "Collapsed" :!label _label)
        (Variables|Default|SetPreviouslyOverlapActor 0)))
    (else
      (goto _label))))

(event Input|KeyboardEvents|LeftCtrl
  (params (Key :type Key%20Structure :default "None"))
  (:Pressed
    (Variables|Default|SetIsCtrlDown true))
  (:Released
    (Variables|Default|SetIsCtrlDown false)))

(fn ConstructionScript
  (|CallParentFunction))

(fn SpawnBuild
  (params (Class :type A%20Builds%20Class%20Reference))
  (if (Utilities|Time|IsValidTimerHandle (Variables|Default|GetDeleteBuild))
    (Utilities|Time|ClearandInvalidateTimerbyHandle (Variables|Default|GetDeleteBuild))
    (bind _itemtodelete (Variables|Default|GetItemToDelete)
      (:then
        (Default|SetAllMaterials _itemtodelete 0 true)
        (Variables|Default|SetItemToDelete 0))
      (:else
        _)))
  (bind _itemtobuild (Variables|Default|GetItemToBuild)
    (:then
      (Default|CancelBuild _itemtobuild))
    (:else
      _))
  (bind (_outhit _returnvalue) (CallFunction|LineTracefromCamera "TraceTypeQuery4"))
  (if _returnvalue
    (bind _returnvalue_2 (Game|SpawnActorfromClass Class (Math|Transform|MakeTransform (.ImpactPoint (|PrepareSpawPosition _outhit)) (.ReturnValue (|PrepareSpawPosition _outhit)) "1.000000,1.000000,1.000000") "Undefined" "MultiplyWithRoot" 0 0 0))
    (Variables|Default|SetItemToBuild _returnvalue_2)
    (bind _returnvalue_3 (Utilities|Time|SetTimerbyFunctionName 0 "MovingBuild" 0.05 true))
    (Variables|Default|SetMoveBuild _returnvalue_3)
    (return)))

(fn MovingBuild
  (bind (_outhit _returnvalue) (CallFunction|LineTracefromCamera "TraceTypeQuery1"))
  (if _returnvalue
    (Default|UpdateLocation (Variables|Default|GetItemToBuild) _outhit)
    (return)))

(fn PlaceBuild
  (if (Default|IsBuildable (Variables|Default|GetItemToBuild))
    (bind _returnvalue (Default|ConfirmBuild (Variables|Default|GetItemToBuild)))
    (if _returnvalue
      (Utilities|Time|ClearandInvalidateTimerbyHandle (Variables|Default|GetMoveBuild))
      (Variables|Default|SetItemToBuild 0)
      (return))))

(fn CancelBuild
  (Default|CancelBuild (Variables|Default|GetItemToBuild))
  (Utilities|Time|ClearandInvalidateTimerbyHandle (Variables|Default|GetMoveBuild))
  (Variables|Default|SetItemToBuild 0)
  (return))

(fn DetermineDelete
  (bind (_outhit _returnvalue) (CallFunction|LineTracefromCamera "TraceTypeQuery3"))
  (if _returnvalue
    (bind _itemtodelete (Variables|Default|GetItemToDelete)
      (:then
        (if (not (== _itemtodelete (.HitActor (Collision|BreakHitResult _outhit))))
          (Default|SetAllMaterials (Variables|Default|GetItemToDelete) 0 true :!label _label)
          (bind _asa_builds (Utilities|Casting|CastToA_Builds (.HitActor (Collision|BreakHitResult _outhit)) :!label _label_2)
            (:then
              (bind _output_get (Variables|Default|SetItemToDelete _asa_builds))
              (Default|SetAllMaterials _output_get "/Game/Game/Assets/Materials/MI_HologramDelete.MI_HologramDelete" false))
            (:CastFailed
              (Variables|Default|SetItemToDelete 0)))))
      (:else
        (goto _label_2)))
    (else
      (bind _itemtodelete_2 (Variables|Default|GetItemToDelete)
        (:then
          (goto _label))
        (:else)))))

(fn LineTracefromCamera
  (params (TraceChannel :type ETraceTypeQuery%20Enum :default "TraceTypeQuery1"))
  (bind _firstpersoncamera (Variables|Default|GetFirstPersonCamera))
  (bind _returnvalue (Transformation|GetWorldLocation _firstpersoncamera))
  (bind (_outhit _returnvalue_2) (Collision|LineTraceByChannel _returnvalue (+ _returnvalue (* (Math|Vector|GetForwardVector _firstpersoncamera) 800)) TraceChannel false (Utilities|Array|MakeArray 0) "None"))
  (return _outhit _returnvalue_2))

(fn PickUpItem
  (params (NewItem :type A%20Items%20Object%20Reference))
  (bind _returnvalue (Default|PickUpItem (Variables|Default|GetAC_Inventory) NewItem))
  (if _returnvalue
    (Actor|DestroyActor NewItem))
  (return _returnvalue))