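; Inventory actor component that stores items as a slot-keyed map of data asset and quantity, up to a maximum size.
; Pickup fills matching stacks up to their max before using an empty slot, with optional duplicate stacks, and a separate check tests for space.
; The inventory input lazily creates and toggles WB_Inventory, whose events update the map.
; Dropped items spawn as A_Items on the surface found by a downward box trace ahead of the owner.
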(event Input|EnhancedActionEvents|EnhancedInputActionIA_Inventory
  (params (ActionValue :type Boolean) (ElapsedSeconds :type Float%20%28double-precision%29) (TriggeredSeconds :type Float%20%28double-precision%29) (InputAction :type Input%20Action%20Object%20Reference :default "/Game/Game/Blueprint/Inputs/IA_Inventory.IA_Inventory"))
  (bind _returnvalue (Game|GetPlayerController 0))
  (:Started
    (Variables|Default|GetAsUmgInventory
      (:then
        _)
      (:else
        (bind _returnvalue_2 (UserInterface|CreateWidget "/Game/Game/Widgets/inventory/WB_Inventory.WB_Inventory_C" 0 (Variables|Default|GetInventory) (Variables|Default|GetMaxSize) (Variables|Default|GetAllowedDuplicates)))
        (Widget|SetVisibility _returnvalue_2 "Collapsed")
        (bind _output_get (Variables|Default|SetAsUmgInventory _returnvalue_2))
        (EventDispatchers|BindEventtoItemAdded (Variables|Default|GetAsUmgInventory) (EventDispatchers|CreateEvent :!event ItemAdded))
        (EventDispatchers|BindEventtoItemDropped (Variables|Default|GetAsUmgInventory) (EventDispatchers|CreateEvent :!event ItemDropped))
        (EventDispatchers|BindEventtoItemRemoved (Variables|Default|GetAsUmgInventory) (EventDispatchers|CreateEvent :!event ItemRemoved))
        (UserInterface|Viewport|AddtoViewport _output_get 0)))
    (Variables|/Script/Engine.PlayerController|SetbShowMouseCursor _returnvalue (not (Widget|IsVisible (Variables|Default|GetAsUmgInventory))))
    (Widget|SetVisibility (Variables|Default|GetAsUmgInventory) (select (Widget|IsVisible (Variables|Default|GetAsUmgInventory)) "Collapsed" "Visible"))
    (Utilities|FlowControl|FlipFlop
      (:A
        (Input|SetInputModeGameandUI _returnvalue (Variables|Default|GetAsUmgInventory) "DoNotLock" true false))
      (:B
        (Input|SetInputModeGameOnly _returnvalue true)))))

(event EventBeginPlay)

(fn PickUpItem
  (params (NewItem :type A%20Items%20Object%20Reference))
  (bind _l_index (LocalVariables|GetL_Index))
  (bind _inventory (Variables|Default|GetInventory))
  (bind _l_index_2 (LocalVariables|GetL_Index))
  (bind (_returnvalue _remainiingquantity) (CallFunction|IsKeyFull _l_index))
  (bind _value (Utilities|Map|Find _inventory _l_index_2))
  (LocalVariables|SetL_QuantityIn (Variables|/Game/Game/Blueprint/A_Items.A_Items_C|GetQuantity NewItem))
  (LocalVariables|SetL_DataAsset (Variables|/Game/Game/Blueprint/A_Items.A_Items_C|GetDataAsset NewItem))
  (while (and (> (LocalVariables|GetL_QuantityIn) 0) (< (LocalVariables|GetL_Index) (Variables|Default|GetMaxSize)))
    (Utilities|FlowControl|Sequence
      (:then_0
        (if _returnvalue
          (if (== (.itemdata (.Value (Utilities|Map|Find (Variables|Default|GetInventory) (LocalVariables|GetL_Index)))) (LocalVariables|GetL_DataAsset))
            (LocalVariables|SetL_FoundSameItem true))
          (else
            (bind _output_get (LocalVariables|SetL_Remaining _remainiingquantity))
            (if (== _output_get -1)
              (if (== -1 (LocalVariables|GetL_EmptyKey))
                (LocalVariables|SetL_EmptyKey (LocalVariables|GetL_Index)))
              (elif (== (.itemdata _value) (LocalVariables|GetL_DataAsset))
                (Utilities|Map|Add (Variables|Default|GetInventory) (LocalVariables|GetL_Index) (Utilities|Struct|MakeS_inventory (+ (.quantity _value) (Math|Integer|Clamp(Integer) (LocalVariables|GetL_QuantityIn) 0 (LocalVariables|GetL_Remaining))) (LocalVariables|GetL_DataAsset)))
                (LocalVariables|SetL_QuantityIn (Math|Integer|Clamp(Integer) (- (LocalVariables|GetL_QuantityIn) (LocalVariables|GetL_Remaining)) 0 (- (LocalVariables|GetL_QuantityIn) (LocalVariables|GetL_Remaining))))
                (LocalVariables|SetL_FoundSameItem true))))))
      (:then_1
        (Math|Integer|IncrementInt (LocalVariables|GetL_Index)))))
  (if (== (LocalVariables|GetL_QuantityIn) 0)
    (return true)
    (elif (and (not (Variables|Default|GetAllowedDuplicates)) (LocalVariables|GetL_FoundSameItem))
      (Default|ModifyQuantity NewItem (LocalVariables|GetL_Remaining))
      (return false)
      (elif (!= (LocalVariables|GetL_EmptyKey) -1)
        (Utilities|Map|Add (Variables|Default|GetInventory) (LocalVariables|GetL_EmptyKey) (Utilities|Struct|MakeS_inventory (LocalVariables|GetL_QuantityIn) (LocalVariables|GetL_DataAsset)))
        (return true)
        (else
          (return false))))))

(fn IsKeyFull
  (params (Key :type Integer))
  (bind _inventory (Variables|Default|GetInventory))
  (bind (_value _returnvalue) (Utilities|Map|Find _inventory Key))
  (bind (_quantity _itemdata) (Utilities|Struct|BreakS_inventory _value))
  (bind _maxstack (Variables|/Game/Game/Blueprint/Items/DataAssets/DA_Items.DA_Items_C|GetMaxStack _itemdata))
  (bind _returnvalue_2 (- _maxstack _quantity))
  (if _returnvalue
    (return (and (== _returnvalue_2 0) (!= _maxstack 0)) _returnvalue_2)
    (else
      (return false -1))))

(fn ItemAdded
  (params (SlotKey :type Integer) (SlotValue :type S%20Inventory%20Structure))
  (Utilities|Map|Add (Variables|Default|GetInventory) SlotKey SlotValue))

(fn ItemDropped
  (params (ItemDropped :type S%20Inventory%20Structure))
  (bind _returnvalue (Components|GetOwner))
  (bind (_quantity _itemdata) (Utilities|Struct|BreakS_inventory ItemDropped))
  (bind _returnvalue_2 (Transformation|GetActorForwardVector _returnvalue))
  (bind _returnvalue_3 (Transformation|GetActorLocation _returnvalue))
  (bind _returnvalue_4 (* _returnvalue_2 3e+02))
  (bind _returnvalue_5 (+ _returnvalue_4 _returnvalue_3))
  (bind (_outhit _returnvalue_6) (Collision|BoxTraceByChannel _returnvalue_5 (- _returnvalue_5 "0.000000,0.000000,500.000000") "15.000000,15.000000,15.000000" "0, 0, 0" "TraceTypeQuery1" false (Utilities|Array|MakeArray (Components|GetOwner)) "None"))
  (if _returnvalue_6
    (Game|SpawnActorfromClass "/Game/Game/Blueprint/A_Items.A_Items_C" (Math|Transform|MakeTransform (.ImpactPoint (Collision|BreakHitResult _outhit)) "0, 0, 0" "1.000000,1.000000,1.000000") "Undefined" "MultiplyWithRoot" 0 _itemdata 0 0.0 _quantity 0)))

(fn ItemRemoved
  (params (Key :type Integer))
  (Utilities|Map|Remove (Variables|Default|GetInventory) Key))

(fn HasPlaceforItem
  (params (struct :type S%20Inventory%20Structure))
  (bind _inventory (Variables|Default|GetInventory))
  (if (> (Variables|Default|GetMaxSize) (Utilities|Map|Length (Variables|Default|GetInventory)))
    (return true)
    (else
      (bind _output_get (LocalVariables|SetL_quantityIn (.quantity struct)))
      (while (and (> _output_get 0) (< (LocalVariables|GetL_Index) (Variables|Default|GetMaxSize)))
        (bind _keys (Utilities|Map|Keys _inventory))
        (if (== (.itemdata struct) (.itemdata (.Value (Utilities|Map|Find _inventory (Utilities|Array|Get(acopy) _keys (LocalVariables|GetL_Index))))))
          (LocalVariables|SetL_quantityIn (- (LocalVariables|GetL_quantityIn) (- (Variables|/Game/Game/Blueprint/Items/DataAssets/DA_Items.DA_Items_C|GetMaxStack (.itemdata (.Value (Utilities|Map|Find _inventory (Utilities|Array|Get(acopy) _keys (LocalVariables|GetL_Index)))))) (.quantity (.Value (Utilities|Map|Find _inventory (Utilities|Array|Get(acopy) _keys (LocalVariables|GetL_Index))))))))))
      (return (<= (LocalVariables|GetL_quantityIn) 0)))))